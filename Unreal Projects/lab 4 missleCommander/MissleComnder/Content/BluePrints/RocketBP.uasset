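; RocketBP is a rocket hazard that moves vertically at FallSpeed with looping travel sound and explodes on hitting the player, base, arrows or worldSpawner.
; Mesh overlaps feed HandleCollision, where arrow hits spawn a coin and add score, while player or base hits subtract health through gameModeBP.
; All handled hits share a one-time death sequence that hides the mesh and switches effects and sounds, then Tick destroys the actor once the explosion finishes.
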(event `self.ReceiveTick`
  (params (DeltaSeconds :type "Float (single-precision)"))
  (bind _movesound (`self.MoveSound`))
  (if (`self.Dead`)
    (if (not (`ActorComponent.IsActive` (`self.Explosion`)))
      (`self.K2_DestroyActor`)
      (`KismetSystemLibrary.PrintString` "Boom"))
    (else
      (`self.K2_AddActorWorldOffset` (`KismetMathLibrary.MakeVector` 0.0 0.0 (* DeltaSeconds (`self.FallSpeed`))))
      (if (not (`AudioComponent.IsPlaying` _movesound))
        (`AudioComponent.Play` _movesound 0.0)))))

(event `self.RocketMesh.OnComponentBeginOverlap`
  (params (OverlappedComponent :type "PrimitiveComponent Object Reference") (OtherActor :type "Actor Object Reference") (OtherComp :type "PrimitiveComponent Object Reference") (OtherBodyIndex :type Integer) (bFromSweep :type Boolean) (SweepResult :type "HitResult Structure (by ref)"))
  (`self.HandleCollision` OtherActor))

(fn `HandleCollision`
  (params (otherObj :type "Actor Object Reference"))
  (bind _movesound (`self.MoveSound`))
  ;[1 0.2598 0.4305] If other object hit, destroy this rocket
  (cast `worldSpawner` otherObj
    (:`then`
      _)
    (:`CastFailed`
      ;[1 1 1] Spawn Coin and add points if hit by arrow
      (cast `/Game/BluePrints/arrowBP` otherObj
        (:`then`
          (`self.SpawnCoinAndAddPoints`))
        (:`CastFailed`
          ;[0.2443 0.2126 1] If Player or base is hit, subtract health
          (cast `/Game/BluePrints/BaseBP` otherObj
            (:`then`
              _)
            (:`CastFailed`
              (cast `/Game/BluePrints/PlayerBP` otherObj)))
          (bind _asgame_mode_bp (cast `/Game/BluePrints/gameModeBP` (`GameplayStatics.GetGameMode`)))
          (`/Game/BluePrints/gameModeBP.SubHealth` _asgame_mode_bp (`self.RocketDamage`))))))
  (if (not (`self.Dead`))
    (`ActorComponent.Activate` (`self.Explosion`) true)
    (set `self.Dead` true)
    (`SceneComponent.SetVisibility` (`self.RocketMesh`) false false)
    (`ActorComponent.Deactivate` (`self.RocketTravel`))
    (`ActorComponent.Activate` (`self.DeadSound`) true)
    (`AudioComponent.Stop` _movesound)
    (`ActorComponent.Deactivate` _movesound)))

(fn `SpawnCoinAndAddPoints`
  (`|SpawnActorFromClass` "/Game/BluePrints/CoinBP.CoinBP_C" (`SceneComponent.K2_GetComponentToWorld` (`self.RocketMesh`)) "AdjustIfPossibleButAlwaysSpawn" "OverrideRootScale" null null)
  (bind _asgame_mode_bp (cast `/Game/BluePrints/gameModeBP` (`GameplayStatics.GetGameMode`)))
  (`/Game/BluePrints/gameModeBP.AddToScore` _asgame_mode_bp (`self.RocketValue`)))

(fn `UserConstructionScript`
  (`SceneComponent.K2_SetWorldRotation` (`self.RocketMesh`) (struct :`Pitch` 180.0) false false))