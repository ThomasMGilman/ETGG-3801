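; Game mode Blueprint that owns the HUD and menu widgets and tracks health, score and money.
; On BeginPlay it layers MenuUI over InGameUI, shows the cursor, freezes time through global time dilation and plays the title animation.
; Its functions update the HUD: health scales the bar horizontally, AddToScore replaces rather than increments the score, money accumulates.
; DisplayEnterText toggles a prompt's opacity only for PlayerBP actors.
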(event `self.ReceiveBeginPlay`
  (bind _menu_ui (`self.Menu_UI`))
  (bind _returnvalue (`|CreateWidget` "/Game/UserOverlay/InGameUI.InGameUI_C"))
  (bind _output_get (set `self.InGame_UI` _returnvalue))
  (`UserWidget.AddToViewport` _output_get 0)
  (bind _returnvalue_2 (`|CreateWidget` "/Game/Menu/menuUI.menuUI_C"))
  (bind _output_get_2 (set `self.Menu_UI` _returnvalue_2))
  (`UserWidget.AddToViewport` _output_get_2 1)
  (set `PlayerController.bShowMouseCursor` true (`GameplayStatics.GetPlayerController` 0))
  (`GameplayStatics.SetGlobalTimeDilation` 0.0)
  (`UserWidget.PlayAnimation` _menu_ui (`/Game/Menu/menuUI.TitleAnimation` _menu_ui) 0.0 1 "Forward" 0.25))

(fn `AddToScore`
  (params (NewScore :type Integer))
  (bind _output_get (set `self.CurrentScore` NewScore))
  (`TextBlock.SetText` (`/Game/UserOverlay/InGameUI.Score_Val` (`self.InGame_UI`)) (`KismetTextLibrary.Conv_StringToText` (`KismetStringLibrary.Conv_IntToString` _output_get))))

(fn `AppendMoney`
  (params (Cost :type Integer))
  (bind _output_get (set `self.CurrentMoney` (+ (`self.CurrentMoney`) Cost)))
  (`TextBlock.SetText` (`/Game/UserOverlay/InGameUI.Money_Val` (`self.InGame_UI`)) (`KismetTextLibrary.Conv_StringToText` (`KismetStringLibrary.Conv_IntToString` _output_get))))

(fn `Display_enterText`
  (params (display :type Boolean) (other :type "Actor Object Reference"))
  (bind _entertext (`/Game/UserOverlay/InGameUI.enterText` (`self.InGame_UI`)))
  (`KismetSystemLibrary.PrintString` "Calling")
  (cast `/Game/BluePrints/PlayerBP` other)
  (if display
    (`TextBlock.SetOpacity` _entertext 75.0)
    (else
      (`TextBlock.SetOpacity` _entertext 0.0))))

(fn `SetHealth`
  (params (PercentHealth :type "Float (double-precision)"))
  (`Widget.SetRenderScale` (`/Game/UserOverlay/InGameUI.HealthBar` (`self.InGame_UI`)) (`KismetMathLibrary.MakeVector2D` PercentHealth 1.0)))

(fn `SubHealth`
  (params (damage :type "Float (double-precision)"))
  (bind _output_get (set `self.CurrentHealth` (- (`self.CurrentHealth`) damage)))
  (`self.SetHealth` _output_get))

(fn `UserConstructionScript`)