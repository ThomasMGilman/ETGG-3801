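; Player Blueprint that walks, sprints, jumps, and can occupy turrets or bases to fire arrows.
; Axis inputs drive manual actor offsets, mouse look and walk animation, with walking disabled inside buildings.
; Tick applies hand-rolled jump and gravity velocities, while world-spawner overlaps snap the mesh to ground height.
; Overlaps also handle coins and record nearby buildings for entry via the game mode, though both events pass Colliding false, bypassing coin pickup.
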(event `self.ReceiveBeginPlay`
  (set `self.health` (`self.max_health`)))

(event `self.ReceiveTick`
  (params (DeltaSeconds :type "Float (single-precision)"))
  (bind _dissphere (`self.disSphere`))
  (`self.isFalling` DeltaSeconds)
  (if (`self.InBuilding`)
    (`SceneComponent.SetVisibility` _dissphere true false)
    (else
      (`SceneComponent.SetVisibility` _dissphere false false))))

(event `InputAxis|Horizontal`
  (params (AxisValue :type "Float (single-precision)"))
  ;[1 0.1032 0.989] PlayerMovement
  (if (not (`self.InBuilding`))
    (bind _varout (`self.getSpeed_Multiplier` AxisValue))
    (`self.K2_AddActorLocalOffset` (* (`KismetMathLibrary.MakeVector` _varout (stale `InputAxis|Vertical` _result)) (`self.SpeedMultiplier`)) :!label _label)
    ;[0.6988 1 0.4973] Play The Specified Animation
    (bind _asplayer_anim_graph (cast `/Game/Animation/PlayerAnimGraph` (`SkeletalMeshComponent.GetAnimInstance` (`self.PlayerMesh`))))
    (set `/Game/Animation/PlayerAnimGraph.walkingAmount` (* (`KismetMathLibrary.FMax` (`KismetMathLibrary.Abs` _varout) (`KismetMathLibrary.Abs` (stale `InputAxis|Vertical` _result))) 100.0) _asplayer_anim_graph)))

(event `InputAxis|Vertical`
  (params (AxisValue :type "Float (single-precision)"))
  ;[1 0.1032 0.989] PlayerMovement
  (if (not (`self.InBuilding`))
    (bind _varout (`self.getSpeed_Multiplier` AxisValue))
    (bind _result (`/Engine/EditorBlueprintResources/StandardMacros.NegateFloat` _varout)
      (:`  `
        (goto _label)))))

(event `InputAction|Fire`
  (params (Key :type "Key Structure"))
  ;[1 1 1] InputActions
  (:`Pressed`
    (`self.fireArrow`)))

(event `InputAction|Sprint`
  (params (Key :type "Key Structure"))
  ;[1 1 1] InputActions
  (:`Pressed`
    (set `self.SpeedMultiplier` 4.0))
  (:`Released`
    (set `self.SpeedMultiplier` 1.0)))

(event `InputAxis|MouseX`
  (params (AxisValue :type "Float (single-precision)"))
  ;[1 1 1] InputActions
  (`self.K2_AddActorLocalRotation` (`KismetMathLibrary.MakeRotator` 0.0 0.0 AxisValue)))

(event `InputAxis|MouseY`
  (params (AxisValue :type "Float (single-precision)"))
  ;[1 1 1] InputActions
  (`SceneComponent.K2_AddLocalRotation` (`self.SpringArm`) (`KismetMathLibrary.MakeRotator` 0.0 AxisValue) false false))

(event `Key|Escape`
  (params (Key :type "Key Structure"))
  ;[1 1 1] InputActions
  (:`Pressed`
    (bind _asgame_mode_bp (cast `/Game/BluePrints/gameModeBP` (`GameplayStatics.GetGameMode`)))
    (`/Game/Menu/menuUI.SetVisible` (`/Game/BluePrints/gameModeBP.Menu_UI` _asgame_mode_bp))
    (set `PlayerController.bShowMouseCursor` true (`GameplayStatics.GetPlayerController` 0))))

(event `InputAction|Jump`
  (params (Key :type "Key Structure"))
  ;[1 1 1] InputActions
  (:`Pressed`
    (`self.Jump`)))

(event `InputAction|Enter`
  (params (Key :type "Key Structure"))
  ;[1 1 1] InputActions
  (:`Pressed`
    (`self.InteractWithBase`)))

(event `self.PlayerMesh.OnComponentBeginOverlap`
  (params (OverlappedComponent :type "PrimitiveComponent Object Reference") (OtherActor :type "Actor Object Reference") (OtherComp :type "PrimitiveComponent Object Reference") (OtherBodyIndex :type Integer) (bFromSweep :type Boolean) (SweepResult :type "HitResult Structure (by ref)"))
  ;[1 1 1] Collision
  (`self.handle_Collision` OtherActor))

(event `self.PlayerMesh.OnComponentEndOverlap`
  (params (OverlappedComponent :type "PrimitiveComponent Object Reference") (OtherActor :type "Actor Object Reference") (OtherComp :type "PrimitiveComponent Object Reference") (OtherBodyIndex :type Integer))
  ;[1 1 1] Collision
  (`self.handle_Collision` OtherActor))

(fn `fireArrow`
  (if (`self.InBuilding`)
    (bind _returnvalue (`|SpawnActorFromClass` "/Game/BluePrints/arrowBP.arrowBP_C" (`KismetMathLibrary.MakeTransform` (`self.K2_GetActorLocation`) (`KismetMathLibrary.MakeRotator` (.roll (`SceneComponent.K2_GetComponentRotation` (`self.PlayerCamer`))) (.pitch (`SceneComponent.K2_GetComponentRotation` (`self.PlayerCamer`))) (- (.yaw (`SceneComponent.K2_GetComponentRotation` (`self.PlayerCamer`))) 0.0)) (0.1 0.1 0.1)) "Undefined" "OverrideRootScale" null null))
    (set `/Game/BluePrints/arrowBP.distance` (`self.forwardDis`) _returnvalue)))

(fn `getSpeed_Multiplier`
  (params (varToMultiply :type "Float (double-precision)"))
  (returns (varOut :type "Float (double-precision)"))
  (return (* varToMultiply (`self.moveSpeed`) (`GameplayStatics.GetWorldDeltaSeconds`))))

(fn `handle_Collision`
  (params (otherObject :type "Actor Object Reference") (Colliding :type Boolean))
  (bind _coinworth (`self.CoinWorth`))
  ;[1 1 1] Ground Collision, stop falling
  (bind _asworld_spawner (cast `worldSpawner` otherObject)
    (:`then`
      (bind (_origin _boxextent) (`self.GetActorBounds` _asworld_spawner false))
      ;[0.5071 1 0.3153] Offset Players position by the difference between the ground and players height
      (`SceneComponent.K2_AddWorldOffset` (`self.PlayerMesh`) (`KismetMathLibrary.MakeVector` 0.0 0.0 (- (+ (.z _origin) (.z _boxextent) 0.0) (.z (`SceneComponent.K2_GetComponentLocation` (`self.PlayerMesh`))))) false false)
      ;[1 1 1] Player is on ground
      (set `self.JumpVelocity` 0.0)
      (set `self.FallingVelocity` 0.0))
    (:`CastFailed`
      ;[1 0.9075 0.7618] Increase Score by CoinWorth
      (bind _ascoin_bp (cast `/Game/BluePrints/CoinBP` otherObject)
        (:`then`
          (if Colliding
            (`ActorComponent.K2_DestroyComponent` (`/Game/BluePrints/CoinBP.CoinMesh` _ascoin_bp))
            (bind _asgame_mode_bp (cast `/Game/BluePrints/gameModeBP` (`GameplayStatics.GetGameMode`)))
            (`/Game/BluePrints/gameModeBP.AddToScore` _asgame_mode_bp (+ (`/Game/BluePrints/gameModeBP.CurrentScore` _asgame_mode_bp) _coinworth))
            (`/Game/BluePrints/gameModeBP.AppendMoney` _asgame_mode_bp _coinworth)))
        (:`CastFailed`
          (bind _asturret_bp (cast `/Game/BluePrints/TurretBP` otherObject)
            (:`then`
              (if Colliding
                (set `self.BuildingCollidingWith` (make `/Game/BluePrints/CollisionStruct` true _asturret_bp))
                (else
                  (set `self.BuildingCollidingWith` (make `/Game/BluePrints/CollisionStruct` false _asturret_bp)))))
            (:`CastFailed`
              (bind _asbase_bp (cast `/Game/BluePrints/BaseBP` otherObject))
              (if Colliding
                (set `self.BuildingCollidingWith` (make `/Game/BluePrints/CollisionStruct` true _asbase_bp))
                (else
                  (set `self.BuildingCollidingWith` (make `/Game/BluePrints/CollisionStruct` false _asbase_bp)))))))))))

(fn `InteractWithBase`
  (bind _returnvalue (`GameplayStatics.GetGameMode`))
  (bind (_colliding _otherobj) (break `/Game/BluePrints/CollisionStruct` (`self.BuildingCollidingWith`)))
  (if _colliding
    _
    (else
      _))
  (bind _asturret_bp (cast `/Game/BluePrints/TurretBP` _otherobj)
    (:`then`
      (bind _occupiedstate (`/Game/BluePrints/TurretBP.OccupyBuilding` _asturret_bp self))
      (bind _output_get (set `self.InBuilding` _occupiedstate))
      (bind _asgame_mode_bp (cast `/Game/BluePrints/gameModeBP` _returnvalue))
      (`/Game/BluePrints/gameModeBP.EnterBuilding` _asgame_mode_bp false _output_get))
    (:`CastFailed`
      (bind _asbase_bp (cast `/Game/BluePrints/BaseBP` _otherobj))
      (bind _occupiedstate_2 (`/Game/BluePrints/BaseBP.OccupyBuilding` _asbase_bp self))
      (bind _output_get_2 (set `self.InBuilding` _occupiedstate_2))
      (bind _asgame_mode_bp_2 (cast `/Game/BluePrints/gameModeBP` _returnvalue))
      (`/Game/BluePrints/gameModeBP.EnterBuilding` _asgame_mode_bp_2 true _output_get_2))))

(fn `isFalling`
  (params (time :type "Float (double-precision)"))
  ;[1 1 1] If Player is falling, incriment falling velocity otherwise reset it. Change players location based on velocity if falling
  (if (`self.Falling`)
    (bind _output_get (set `self.FallingVelocity` (+ (`self.FallingVelocity`) (* time (`self.GravityConstant`)))))
    (else
      (bind _output_get_2 (set `self.FallingVelocity` 0.0))))
  ;[1 1 1] Update Jump Velocity by multiplying it by elapsed time
  (bind _output_get_3 (set `self.JumpVelocity` (* (`self.JumpVelocity`) 1.0)))
  ;[1 1 1] add world offset by Falling velocity + Jump velocity
  (`self.K2_AddActorWorldOffset` (`KismetMathLibrary.MakeVector` 0.0 0.0 (+ _output_get_3 (+ _output_get _output_get_2))) true))

(fn `Jump`
  (if (<= (`self.JumpVelocity`) 0.0)
    (set `self.JumpVelocity` (`self.JumpAmount`))))

(fn `UserConstructionScript`)