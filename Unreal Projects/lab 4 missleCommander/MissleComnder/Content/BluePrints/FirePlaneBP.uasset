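; FirePlaneBP is an actor that periodically spawns RocketBP actors at random points across a large square area.
; Tick counts SpawnCountDown down by delta time, then calls SpawnRocket and resets the timer to SpawnRate.
; SpawnRocket offsets FirePlaneMesh's world location by random X and Y within hardcoded symmetric bounds, keeping the mesh's height.
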(event `self.ReceiveTick`
  (params (DeltaSeconds :type "Float (single-precision)"))
  (bind _spawncountdown (`self.SpawnCountDown`))
  (if (<= _spawncountdown 0.0)
    (`self.SpawnRocket`)
    (set `self.SpawnCountDown` (`self.SpawnRate`))
    (else
      (set `self.SpawnCountDown` (- _spawncountdown DeltaSeconds)))))

(fn `SpawnRocket`
  (bind _returnvalue (/ (* 60.0 201.0) 2.0))
  (bind _returnvalue_2 (* _returnvalue -1.0))
  (`|SpawnActorFromClass` "/Game/BluePrints/RocketBP.RocketBP_C" (`KismetMathLibrary.Conv_VectorToTransform` (+ (`SceneComponent.K2_GetComponentLocation` (`self.FirePlaneMesh`)) (`KismetMathLibrary.MakeVector` (`KismetMathLibrary.RandomFloatInRange` _returnvalue_2 _returnvalue) (`KismetMathLibrary.RandomFloatInRange` _returnvalue_2 _returnvalue)))) "Undefined" "OverrideRootScale" null null))

(fn `UserConstructionScript`)