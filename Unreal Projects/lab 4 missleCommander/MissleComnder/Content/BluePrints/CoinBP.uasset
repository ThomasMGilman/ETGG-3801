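; Coin pickup actor that falls, spins, and disappears when the player touches it.
; Tick applies hand-rolled gravity through unswept world offsets and rotates the coin, with the Clockwise flag choosing positive pitch or negative roll.
; Overlapping a worldSpawner stops the fall, while overlapping PlayerBP destroys only the mesh component, with no score logic.
; The construction script shrinks the mesh to a fixed scale.
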(event `self.ReceiveTick`
  (params (DeltaSeconds :type "Float (single-precision)"))
  (`self.isFalling` DeltaSeconds)
  (`self.Rotate` DeltaSeconds))

(event `self.CoinMesh.OnComponentBeginOverlap`
  (params (OverlappedComponent :type "PrimitiveComponent Object Reference") (OtherActor :type "Actor Object Reference") (OtherComp :type "PrimitiveComponent Object Reference") (OtherBodyIndex :type Integer) (bFromSweep :type Boolean) (SweepResult :type "HitResult Structure (by ref)"))
  (cast `worldSpawner` OtherActor
    (:`then`
      (set `self.Falling` false))
    (:`CastFailed`
      (cast `/Game/BluePrints/PlayerBP` OtherActor)
      (`ActorComponent.K2_DestroyComponent` (`self.CoinMesh`)))))

(fn `isFalling`
  (params (Time :type "Float (double-precision)"))
  ;[1 1 1] If Player is falling, incriment falling velocity otherwise reset it. Change players location based on velocity if falling
  (if (`self.Falling`)
    (bind _output_get (set `self.FallingVelocity` (+ (`self.FallingVelocity`) (* Time (`self.GravityConstant`)))))
    (`self.K2_AddActorWorldOffset` (`KismetMathLibrary.MakeVector` 0.0 0.0 _output_get))
    (else
      (set `self.FallingVelocity` 0.0))))

(fn `Rotate`
  (params (Time :type "Float (double-precision)"))
  (bind _returnvalue (* Time (`self.RotationSpeed`)))
  (if (`self.Clockwise`)
    (`self.K2_AddActorLocalRotation` (`KismetMathLibrary.MakeRotator` 0.0 _returnvalue))
    (else
      (`self.K2_AddActorLocalRotation` (`KismetMathLibrary.MakeRotator` (* _returnvalue -1.0))))))

(fn `UserConstructionScript`
  (`SceneComponent.SetWorldScale3D` (`self.CoinMesh`) (0.25 0.25 0.25)))