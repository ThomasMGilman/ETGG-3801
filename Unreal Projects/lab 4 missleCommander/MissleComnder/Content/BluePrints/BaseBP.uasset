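; BaseBP is a building that the player can occupy when in range of its mesh.
; BaseMesh overlap begin and end toggle the enter text through gameModeBP and track it in ShowingText, with no filter on the overlapping actor.
; OccupyBuilding occupies only while the text is showing, hiding the prompt, and otherwise clears occupancy, so calling it when occupied vacates the building; it returns the resulting state.
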(event `self.BaseMesh.OnComponentBeginOverlap`
  (params (OverlappedComponent :type "PrimitiveComponent Object Reference") (OtherActor :type "Actor Object Reference") (OtherComp :type "PrimitiveComponent Object Reference") (OtherBodyIndex :type Integer) (bFromSweep :type Boolean) (SweepResult :type "HitResult Structure (by ref)"))
  (bind _asgame_mode_bp (cast `/Game/BluePrints/gameModeBP` (`GameplayStatics.GetGameMode`)))
  (`/Game/BluePrints/gameModeBP.Display_enterText` _asgame_mode_bp true OtherActor)
  (set `self.ShowingText` true))

(event `self.BaseMesh.OnComponentEndOverlap`
  (params (OverlappedComponent :type "PrimitiveComponent Object Reference") (OtherActor :type "Actor Object Reference") (OtherComp :type "PrimitiveComponent Object Reference") (OtherBodyIndex :type Integer))
  (bind _asgame_mode_bp (cast `/Game/BluePrints/gameModeBP` (`GameplayStatics.GetGameMode`)))
  (`/Game/BluePrints/gameModeBP.Display_enterText` _asgame_mode_bp false OtherActor)
  (set `self.ShowingText` false))

(fn `OccupyBuilding`
  (params (playerActor :type "/Game/BluePrints/PlayerBP Object Reference"))
  (returns (OccupiedState :type Boolean))
  (bind _occupiedbyplayer (`self.OccupiedByPlayer`))
  ;[1 1 1] Check if building is occupied by player, if not and text is showing, occupy building, otherwise return false
  (if _occupiedbyplayer
    (set `self.OccupiedByPlayer` false :!label _label)
    (elif (`self.ShowingText`)
      (set `self.OccupiedByPlayer` true)
      (bind _asgame_mode_bp (cast `/Game/BluePrints/gameModeBP` (`GameplayStatics.GetGameMode`)))
      (`/Game/BluePrints/gameModeBP.Display_enterText` _asgame_mode_bp false playerActor)
      (else
        (goto _label))))
  (return _occupiedbyplayer))

(fn `UserConstructionScript`)