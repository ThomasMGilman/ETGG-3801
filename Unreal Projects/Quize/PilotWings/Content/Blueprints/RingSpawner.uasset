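; RingSpawner fills the level with a vertical series of RingBP actors when play begins.
; BeginPlay loops SpawnRing until NumRings runs out, placing each ring at a random X and Y within set bounds.
; Height is RingOffsetZ times the remaining count, so rings spawn from the highest down.
; A coin flip gates each attempt, but only successful flips decrement the count, so it does not reduce the total.
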(event `self.ReceiveBeginPlay`
  (while (> (`self.numRings`) 0.0)
    (`self.SpawnRing`)))

(fn `SpawnRing`
  (if (not (== (`KismetMathLibrary.RandomIntegerInRange` 0 1) 0))
    (`|SpawnActorFromClass` "/Game/Blueprints/RingBP.RingBP_C" (`KismetMathLibrary.MakeTransform` (`KismetMathLibrary.MakeVector` (`KismetMathLibrary.RandomFloatInRange` (`self.minX`) (`self.maxX`)) (`KismetMathLibrary.RandomFloatInRange` (`self.minY`) (`self.maxY`)) (* (`self.ringOffsetZ`) (`self.numRings`)))) "Undefined" "OverrideRootScale" null null)
    (set `self.numRings` (- (`self.numRings`) 1.0))))

(fn `UserConstructionScript`)