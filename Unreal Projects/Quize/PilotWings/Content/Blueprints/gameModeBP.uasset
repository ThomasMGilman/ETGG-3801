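; Game mode Blueprint that owns the HUD and menu widgets and tracks the player's score.
; On BeginPlay it creates both widgets with the menu layered on top, shows the cursor, freezes the game through zero global time dilation and plays the title animation.
; Its functions push score and truncated speed values to the HUD, and on game over pass the final score to the menu and show the cursor.
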(event `self.ReceiveBeginPlay`
  (`self.setGamemode`))

(fn `AddToScore`
  (params (PointsToAdd :type Integer))
  (bind _output_get (set `self.CurrentScore` (+ (`self.CurrentScore`) PointsToAdd)))
  (`TextBlock.SetText` (`/Game/InGameUI/InGameUI.Score_Val` (`self.In Game UI`)) (`KismetTextLibrary.Conv_StringToText` (`KismetStringLibrary.Conv_IntToString` _output_get))))

(fn `GameOver`
  (bind _menu_ui (`self.Menu_UI`))
  (`/Game/Menu/menuUI.GameOver` _menu_ui (`self.CurrentScore`))
  (set `PlayerController.bShowMouseCursor` true (`GameplayStatics.GetPlayerController` 0))
  (set `/Game/Menu/menuUI.gameOv` true _menu_ui))

(fn `setGamemode`
  (bind _menu_ui (`self.Menu_UI`))
  (bind _returnvalue (`|CreateWidget` "/Game/InGameUI/InGameUI.InGameUI_C"))
  (bind _output_get (set `self.In Game UI` _returnvalue))
  (`UserWidget.AddToViewport` _output_get 0)
  (bind _returnvalue_2 (`|CreateWidget` "/Game/Menu/menuUI.menuUI_C"))
  (bind _output_get_2 (set `self.Menu_UI` _returnvalue_2))
  (`UserWidget.AddToViewport` _output_get_2 1)
  (set `PlayerController.bShowMouseCursor` true (`GameplayStatics.GetPlayerController` 0))
  (`GameplayStatics.SetGlobalTimeDilation` 0.0)
  (`UserWidget.PlayAnimation` _menu_ui (`/Game/Menu/menuUI.TitleAnimation` _menu_ui) 0.0 1 "Forward" 0.25))

(fn `setSpeed`
  (params (Speed :type "Float (double-precision)"))
  (`TextBlock.SetText` (`/Game/InGameUI/InGameUI.Speed` (`self.In Game UI`)) (`KismetTextLibrary.Conv_Int64ToText` (`KismetMathLibrary.FTrunc64` Speed))))

(fn `UserConstructionScript`)