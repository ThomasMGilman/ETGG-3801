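; PersonBP is a person Blueprint with a skeletal mesh that starts on a looping idle animation at BeginPlay.
; Pressing E flips the IsWalking flag and plays animations directly on the mesh.
; The branch condition is fixed to true rather than reading IsWalking, so E always starts the looping walk animation and the return to idle never runs.
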(event `self.ReceiveBeginPlay`
  (`SkeletalMeshComponent.PlayAnimation` (`self.SkeletalMesh`) "/Game/Animation/Anim_Armature_Idle.Anim_Armature_Idle" true))

(event `Key|E`
  (params (Key :type "Key Structure"))
  (:`Pressed`
    (set `self.IsWalking` (not (`self.IsWalking`)))
    (if true
      (`SkeletalMeshComponent.PlayAnimation` (`self.SkeletalMesh`) "/Game/Animation/Anim_Armature_Walk.Anim_Armature_Walk" true)
      (else
        (`SkeletalMeshComponent.PlayAnimation` (`self.SkeletalMesh`) "/Game/Animation/Anim_Armature_Idle.Anim_Armature_Idle" true)))))

(fn `UserConstructionScript`)