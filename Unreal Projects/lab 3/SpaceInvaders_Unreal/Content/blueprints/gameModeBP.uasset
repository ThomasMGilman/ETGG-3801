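; Game mode Blueprint that sets up the in-game HUD and the title menu and acts as the update point for health and score display.
; BeginPlay layers MenuUI over InGameUI, shows the cursor, sets global time dilation to zero and plays the title animation slowly.
; SetHealth scales the health bar horizontally by the given value.
; AddToScore replaces CurrentScore with the passed value, despite its name, and refreshes the score text.
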(event `self.ReceiveBeginPlay`
  (bind _menu_ui (`self.Menu_UI`))
  (bind _returnvalue (`|CreateWidget` "/Game/UIElements/InGameUI.InGameUI_C"))
  (bind _output_get (set `self.In Game_UI` _returnvalue))
  (`UserWidget.AddToViewport` _output_get 0)
  (bind _returnvalue_2 (`|CreateWidget` "/Game/menu/menuUI.menuUI_C"))
  (bind _output_get_2 (set `self.Menu_UI` _returnvalue_2))
  (`UserWidget.AddToViewport` _output_get_2 1)
  (set `PlayerController.bShowMouseCursor` true (`GameplayStatics.GetPlayerController` 0))
  (`GameplayStatics.SetGlobalTimeDilation` 0.0)
  (`UserWidget.PlayAnimation` _menu_ui (`/Game/menu/menuUI.TitleAnimation` _menu_ui) 0.0 1 "Forward" 0.25))

(fn `AddToScore`
  (params (NewScore :type Integer))
  (bind _output_get (set `self.CurrentScore` NewScore))
  (`TextBlock.SetText` (`/Game/UIElements/InGameUI.Score_Val` (`self.In Game_UI`)) (`KismetTextLibrary.Conv_StringToText` (`KismetStringLibrary.Conv_IntToString` _output_get))))

(fn `SetHealth`
  (params (PercentHealth :type "Float (double-precision)"))
  (`Widget.SetRenderScale` (`/Game/UIElements/InGameUI.HealthBar` (`self.In Game_UI`)) (`KismetMathLibrary.MakeVector2D` PercentHealth 1.0)))

(fn `UserConstructionScript`)